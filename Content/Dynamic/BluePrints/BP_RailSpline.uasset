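; Rail actor that bends meshes along a spline to form a track, with no runtime logic.
; The construction script fits nine pre-placed SplineMesh components to consecutive segments between the first ten spline points, copying each point's location and tangent.
; Segments are hard-wired rather than looped or spawned, so further points get no mesh.
; Point data is read in world space and passed directly to SetStartAndEnd, which interprets it in component-local space.
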(event EventBeginPlay)

(event Collision|EventActorBeginOverlap
  (params (OtherActor :type Actor%20Object%20Reference)))

(event EventTick
  (params (DeltaSeconds :type Float%20%28single-precision%29)))

(fn ConstructionScript
  (bind _spline (Variables|Default|GetSpline))
  (bind (_location _tangent) (Spline|GetLocationandTangentatSplinePoint _spline 4 "World"))
  (bind (_location_2 _tangent_2) (Spline|GetLocationandTangentatSplinePoint _spline 0 "World"))
  (bind (_location_3 _tangent_3) (Spline|GetLocationandTangentatSplinePoint _spline 1 "World"))
  (bind (_location_4 _tangent_4) (Spline|GetLocationandTangentatSplinePoint _spline 2 "World"))
  (bind (_location_5 _tangent_5) (Spline|GetLocationandTangentatSplinePoint _spline 3 "World"))
  (bind (_location_6 _tangent_6) (Spline|GetLocationandTangentatSplinePoint _spline 5 "World"))
  (bind (_location_7 _tangent_7) (Spline|GetLocationandTangentatSplinePoint _spline 6 "World"))
  (bind (_location_8 _tangent_8) (Spline|GetLocationandTangentatSplinePoint _spline 9 "World"))
  (bind (_location_9 _tangent_9) (Spline|GetLocationandTangentatSplinePoint _spline 7 "World"))
  (bind (_location_10 _tangent_10) (Spline|GetLocationandTangentatSplinePoint _spline 8 "World"))
  (Utilities|FlowControl|Sequence
    (:then_0
      (SplineMesh|SetStartandEnd (Variables|Default|GetSplineMesh) _location_2 _tangent_2 _location_3 _tangent_3 true :!class /Script/Engine.SplineMeshComponent))
    (:then_1
      (SplineMesh|SetStartandEnd (Variables|Default|GetSplineMesh1) _location_3 _tangent_3 _location_4 _tangent_4 true :!class /Script/Engine.SplineMeshComponent))
    (:then_2
      (SplineMesh|SetStartandEnd (Variables|Default|GetSplineMesh2) _location_4 _tangent_4 _location_5 _tangent_5 true :!class /Script/Engine.SplineMeshComponent))
    (:then_3
      (SplineMesh|SetStartandEnd (Variables|Default|GetSplineMesh3) _location_5 _tangent_5 _location _tangent true :!class /Script/Engine.SplineMeshComponent))
    (:then_4
      (SplineMesh|SetStartandEnd (Variables|Default|GetSplineMesh4) _location _tangent _location_6 _tangent_6 true :!class /Script/Engine.SplineMeshComponent))
    (:then_5
      (SplineMesh|SetStartandEnd (Variables|Default|GetSplineMesh5) _location_6 _tangent_6 _location_7 _tangent_7 true :!class /Script/Engine.SplineMeshComponent))
    (:then_6
      (SplineMesh|SetStartandEnd (Variables|Default|GetSplineMesh6) _location_7 _tangent_7 _location_9 _tangent_9 true :!class /Script/Engine.SplineMeshComponent))
    (:then_7
      (SplineMesh|SetStartandEnd (Variables|Default|GetSplineMesh7) _location_9 _tangent_9 _location_10 _tangent_10 true :!class /Script/Engine.SplineMeshComponent))
    (:then_8
      (SplineMesh|SetStartandEnd (Variables|Default|GetSplineMesh8) _location_10 _tangent_10 _location_8 _tangent_8 true :!class /Script/Engine.SplineMeshComponent))))